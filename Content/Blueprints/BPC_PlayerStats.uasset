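; Stats component for the player, dummy and AI characters, tracking health, stamina, XP and level.
; One tick after BeginPlay it casts its owner to set the character type, which selects the HUD or overhead health bar to update.
; Stat functions push changes straight to widgets, with all but DecreaseHealth targeting only the player HUD.
; Decrease functions return true on depletion; leveling up resets XP, scales MaxXP and plays a sound.
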(event `self.ReceiveBeginPlay`
  (`KismetSystemLibrary.DelayUntilNextTick`)
  (`self.InitializePlayerStats`))

(event `InitializePlayerStats`
  (bind _returnvalue (`self.GetOwner`))
  (bind _asbp_third_person_character (cast `/Game/ThirdPerson/Blueprints/BP_ThirdPersonCharacter` _returnvalue)
    (:`then`
      (bind _output_get (set `self.PlayerCharacter BP` _asbp_third_person_character))
      (set `self.IsPlayer` true)
      (set `self.CharacterType` "NewEnumerator0"))
    (:`CastFailed`
      (bind _asbp_dummy (cast `/Game/Blueprints/BP_Dummy` _returnvalue)
        (:`then`
          (set `self.Dummy BP` _asbp_dummy)
          (set `self.CharacterType` "NewEnumerator1"))
        (:`CastFailed`
          (bind _asbp_ai (cast `/Game/AI/BP_AI` _returnvalue))
          (set `self.AI BP` _asbp_ai)
          (set `self.CharacterType` "NewEnumerator2")))
      (set `self.IsPlayer` false)))
  (`ProgressBar.SetPercent` (select `/Game/Blueprints/E_CharacterType` (`self.CharacterType`) :`NewEnumerator0` (`/Game/UI/UWB_HUD.HealthBar` (`/Game/ThirdPerson/Blueprints/BP_ThirdPersonCharacter.HUDWidget` _output_get)) :`NewEnumerator1` (`/Game/UI/UWP_DummyHealthBar.HealthBar` (`/Game/Blueprints/BP_Dummy.HealthBarUI` (`self.Dummy BP`))) :`NewEnumerator2` (`/Game/UI/UWP_DummyHealthBar.HealthBar` (`/Game/AI/BP_AI.HealthBarUI` (`self.AI BP`)))) (/ (`self.Health`) (`self.MaxHealth`)))
  (`TextBlock.SetText` (select `/Game/Blueprints/E_CharacterType` (`self.CharacterType`) :`NewEnumerator0` (`/Game/UI/UWB_HUD.HealthText` (`/Game/ThirdPerson/Blueprints/BP_ThirdPersonCharacter.HUDWidget` (`self.PlayerCharacter BP`))) :`NewEnumerator1` (`/Game/UI/UWP_DummyHealthBar.HealthText` (`/Game/Blueprints/BP_Dummy.HealthBarUI` (`self.Dummy BP`))) :`NewEnumerator2` (`/Game/UI/UWP_DummyHealthBar.HealthText` (`/Game/AI/BP_AI.HealthBarUI` (`self.AI BP`)))) (`KismetTextLibrary.Conv_DoubleToText` (`self.Health`) "HalfToEven"))
  (if (`self.IsPlayer`)
    (`ProgressBar.SetPercent` (`/Game/UI/UWB_HUD.StaminaBar` (`/Game/ThirdPerson/Blueprints/BP_ThirdPersonCharacter.HUDWidget` (`self.PlayerCharacter BP`))) (/ (`self.Stamina`) (`self.MaxStamina`)))
    (`ProgressBar.SetPercent` (`/Game/UI/UWB_HUD.XPBar` (`/Game/ThirdPerson/Blueprints/BP_ThirdPersonCharacter.HUDWidget` (`self.PlayerCharacter BP`))) (/ (`self.XP`) (`self.MaxXP`)))
    (`TextBlock.SetText` (`/Game/UI/UWB_HUD.XPText` (`/Game/ThirdPerson/Blueprints/BP_ThirdPersonCharacter.HUDWidget` (`self.PlayerCharacter BP`))) (`|FormatText` "{XP} / {MaxXP}" (`self.XP`) (`self.MaxXP`)))
    (`TextBlock.SetText` (`/Game/UI/UWB_HUD.LevelText` (`/Game/ThirdPerson/Blueprints/BP_ThirdPersonCharacter.HUDWidget` (`self.PlayerCharacter BP`))) (`KismetTextLibrary.Conv_IntToText` (`self.Level`)))))

(fn `DecreaseHealth`
  (params (Damage :type "Float (double-precision)"))
  (returns (IsDead :type Boolean))
  (if (not (<= (`self.Health`) 0.0))
    (bind _output_get (set `self.Health` (- (`self.Health`) Damage)))
    (`ProgressBar.SetPercent` (select `/Game/Blueprints/E_CharacterType` (`self.CharacterType`) :`NewEnumerator0` (`/Game/UI/UWB_HUD.HealthBar` (`/Game/ThirdPerson/Blueprints/BP_ThirdPersonCharacter.HUDWidget` (`self.PlayerCharacter BP`))) :`NewEnumerator1` (`/Game/UI/UWP_DummyHealthBar.HealthBar` (`/Game/Blueprints/BP_Dummy.HealthBarUI` (`self.Dummy BP`))) :`NewEnumerator2` (`/Game/UI/UWP_DummyHealthBar.HealthBar` (`/Game/AI/BP_AI.HealthBarUI` (`self.AI BP`)))) (/ _output_get (`self.MaxHealth`)))
    (`TextBlock.SetText` (select `/Game/Blueprints/E_CharacterType` (`self.CharacterType`) :`NewEnumerator0` (`/Game/UI/UWB_HUD.HealthText` (`/Game/ThirdPerson/Blueprints/BP_ThirdPersonCharacter.HUDWidget` (`self.PlayerCharacter BP`))) :`NewEnumerator1` (`/Game/UI/UWP_DummyHealthBar.HealthText` (`/Game/Blueprints/BP_Dummy.HealthBarUI` (`self.Dummy BP`))) :`NewEnumerator2` (`/Game/UI/UWP_DummyHealthBar.HealthText` (`/Game/AI/BP_AI.HealthBarUI` (`self.AI BP`)))) (`KismetTextLibrary.Conv_DoubleToText` (`self.Health`) "HalfToEven"))
    (if (<= (`self.Health`) 0.0)
      _
      (else
        (return false))))
  (return true))

(fn `DecreaseStamina`
  (params (StaminaDepleted :type "Float (double-precision)"))
  (returns (NotStaminaLeft :type Boolean))
  (bind _stamina (`self.Stamina`))
  (if (not (<= _stamina 0.0))
    (bind _output_get (set `self.Stamina` (- _stamina StaminaDepleted)))
    (`ProgressBar.SetPercent` (`/Game/UI/UWB_HUD.StaminaBar` (`/Game/ThirdPerson/Blueprints/BP_ThirdPersonCharacter.HUDWidget` (`self.PlayerCharacter BP`))) (/ _output_get (`self.MaxStamina`)))
    (if (<= _output_get 0.0)
      _
      (else
        (return false))))
  (return true))

(fn `IncreaseHealth`
  (params (AddedHealth :type "Float (double-precision)"))
  (bind _maxhealth (`self.MaxHealth`))
  (bind _hudwidget (`/Game/ThirdPerson/Blueprints/BP_ThirdPersonCharacter.HUDWidget` (`self.PlayerCharacter BP`)))
  (bind _output_get (set `self.Health` (+ (`self.Health`) AddedHealth)))
  (if (> _output_get _maxhealth)
    (bind _output_get_2 (set `self.Health` _maxhealth)))
  (`ProgressBar.SetPercent` (`/Game/UI/UWB_HUD.HealthBar` _hudwidget) (/ _output_get_2 (`self.MaxHealth`)))
  (`TextBlock.SetText` (`/Game/UI/UWB_HUD.HealthText` _hudwidget) (`KismetTextLibrary.Conv_DoubleToText` _output_get_2 "HalfToEven")))

(fn `IncreaseLevel`
  (params (AddedLevel :type Integer))
  (set `self.Level` (+ (`self.Level`) AddedLevel))
  (set `self.MaxXP` (`KismetMathLibrary.Conv_IntToDouble` (`KismetMathLibrary.Round` (* (`self.MaxXP`) 1.2))))
  (set `self.XP` 0.0)
  (`TextBlock.SetText` (`/Game/UI/UWB_HUD.LevelText` (`/Game/ThirdPerson/Blueprints/BP_ThirdPersonCharacter.HUDWidget` (`self.PlayerCharacter BP`))) (`KismetTextLibrary.Conv_IntToText` (`self.Level`)))
  (`GameplayStatics.PlaySound2D` "/Game/Audio/UI/SC_LevelUp.SC_LevelUp" 1.0 1.0 0.0 null null))

(fn `IncreaseMaxHealth`
  (params (HealthIncremetion :type "Float (double-precision)"))
  (bind _health (`self.Health`))
  (bind _hudwidget (`/Game/ThirdPerson/Blueprints/BP_ThirdPersonCharacter.HUDWidget` (`self.PlayerCharacter BP`)))
  (bind _output_get (set `self.MaxHealth` (+ (`self.MaxHealth`) HealthIncremetion)))
  (`ProgressBar.SetPercent` (`/Game/UI/UWB_HUD.HealthBar` _hudwidget) (/ _health _output_get))
  (`TextBlock.SetText` (`/Game/UI/UWB_HUD.HealthText` _hudwidget) (`KismetTextLibrary.Conv_DoubleToText` _health "HalfToEven")))

(fn `IncreaseMaxStamina`
  (params (AddedStamina :type "Float (double-precision)"))
  (bind _output_get (set `self.MaxStamina` (+ (`self.MaxStamina`) AddedStamina)))
  (`ProgressBar.SetPercent` (`/Game/UI/UWB_HUD.StaminaBar` (`/Game/ThirdPerson/Blueprints/BP_ThirdPersonCharacter.HUDWidget` (`self.PlayerCharacter BP`))) (/ (`self.Stamina`) _output_get)))

(fn `IncreaseStamina`
  (params (AddedStamina :type "Float (double-precision)"))
  (bind _maxstamina (`self.MaxStamina`))
  (bind _output_get (set `self.Stamina` (+ (`self.Stamina`) AddedStamina)))
  (if (> _output_get _maxstamina)
    (bind _output_get_2 (set `self.Stamina` _maxstamina)))
  (`ProgressBar.SetPercent` (`/Game/UI/UWB_HUD.StaminaBar` (`/Game/ThirdPerson/Blueprints/BP_ThirdPersonCharacter.HUDWidget` (`self.PlayerCharacter BP`))) (/ _output_get_2 (`self.MaxStamina`))))

(fn `IncreaseXP`
  (params (AddedXP :type "Float (double-precision)"))
  (bind _output_get (set `self.XP` (+ (`self.XP`) AddedXP)))
  (if (>= _output_get (`self.MaxXP`))
    (`self.IncreaseLevel` 1))
  (`ProgressBar.SetPercent` (`/Game/UI/UWB_HUD.XPBar` (`/Game/ThirdPerson/Blueprints/BP_ThirdPersonCharacter.HUDWidget` (`self.PlayerCharacter BP`))) (/ (`self.XP`) (`self.MaxXP`)))
  (`TextBlock.SetText` (`/Game/UI/UWB_HUD.XPText` (`/Game/ThirdPerson/Blueprints/BP_ThirdPersonCharacter.HUDWidget` (`self.PlayerCharacter BP`))) (`|FormatText` "{XP} / {MaxXP}" (`self.XP`) (`self.MaxXP`))))