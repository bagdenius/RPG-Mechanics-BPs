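; AI controller for boss enemies that runs the boss behavior tree and manages an on-screen boss health bar.
; BeginPlay starts BT_AI_Boss, while combat activation and deactivation events create and add, or remove and clear, the health bar widget.
; Tick updates the bar's percent from Health over MaxHealth whenever the widget is valid.
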(event `self.ReceiveBeginPlay`
  (`self.RunBehaviorTree` "/Game/AI/Boss/BT_AI_Boss.BT_AI_Boss"))

(event `ActivateBossCombat`
  (bind _returnvalue (`|CreateWidget` "/Game/UI/UWB_BossHealthBar.UWB_BossHealthBar_C"))
  (bind _output_get (set `self.BossHealthBarWidget` _returnvalue))
  (`UserWidget.AddToViewport` _output_get 0))

(event `DeactivateBossCombat`
  (`Widget.RemoveFromParent` (`self.BossHealthBarWidget`))
  (set `self.BossHealthBarWidget` null))

(event `self.ReceiveTick`
  (params (DeltaSeconds :type "Float (single-precision)"))
  (bind _bosshealthbarwidget (`self.BossHealthBarWidget`)
    (:`then`
      (`ProgressBar.SetPercent` (`/Game/UI/UWB_BossHealthBar.HealthBar` _bosshealthbarwidget) (/ (`self.Health`) (`self.MaxHealth`))))
    (:`else`)))

(fn `UserConstructionScript`
  (`parent.UserConstructionScript`))